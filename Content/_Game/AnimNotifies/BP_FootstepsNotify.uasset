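; BP_FootstepsNotify is an animation notify that produces surface-dependent footstep effects for BP_ShooterCharacter.
; On notify, it asks the owning character for its surface type and passes that with the BoneName socket location to FootstepSoundParticle.
; That function maps the surface to a sound and Niagara system, defaulting to metal.
; The particles always spawn, while the sound plays only when ShouldPlaySound is set.
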(fn ReceivedNotify
  (params (MeshComp :type Skeletal%20Mesh%20Component%20Object%20Reference) (Animation :type Anim%20Sequence%20Base%20Object%20Reference) (EventReference :type Anim%20Notify%20Event%20Reference%20Structure%20%28by%20ref%29))
  (bind _bonename (Variables|Default|GetBoneName))
  (bind _returnvalue (Transformation|GetSocketLocation MeshComp _bonename))
  (bind _asbp_shooter_character (Utilities|Casting|CastToBP_ShooterCharacter (Components|GetOwner MeshComp)))
  (bind _returnvalue_2 (Class|ShooterCharacter|GetSurfaceType _asbp_shooter_character))
  (CallFunction|FootstepSoundParticle _returnvalue_2 _returnvalue _returnvalue)
  (return true))

(fn FootstepSoundParticle
  (params (SurfaceType :type EPhysicalSurface%20Enum :default "SurfaceType_Default") (SoundLocation :type Vector) (SpawnLocation :type Vector))
  (LocalVariables|SetSoundSpawnLocation SoundLocation)
  (LocalVariables|SetParticleLocation SpawnLocation)
  (switch Utilities|FlowControl|Switch|SwitchonEPhysicalSurface SurfaceType
    (:SurfaceType_Default
      (LocalVariables|SetSoundVariable "/Game/_Game/Assets/SFX/SFX_MetalFootsteps.SFX_MetalFootsteps")
      (LocalVariables|SetParticleVariable "/Game/A_Surface_Footstep/Niagara_FX/ParticleSystems/PSN_General1_Surface.PSN_General1_Surface"))
    (:SurfaceType1
      (LocalVariables|SetSoundVariable "/Game/_Game/Assets/SFX/SFX_MetalFootsteps.SFX_MetalFootsteps")
      (LocalVariables|SetParticleVariable "/Game/A_Surface_Footstep/Niagara_FX/ParticleSystems/PSN_General1_Surface.PSN_General1_Surface"))
    (:SurfaceType2
      (LocalVariables|SetSoundVariable "/Game/_Game/Assets/SFX/SFX_RockFootsteps.SFX_RockFootsteps")
      (LocalVariables|SetParticleVariable "/Game/A_Surface_Footstep/Niagara_FX/ParticleSystems/PSN_Gravel_Surface.PSN_Gravel_Surface"))
    (:SurfaceType3
      (LocalVariables|SetSoundVariable "/Game/_Game/Assets/SFX/SFX_TileFootstep.SFX_TileFootstep")
      (LocalVariables|SetParticleVariable "/Game/A_Surface_Footstep/Niagara_FX/ParticleSystems/PSN_General2_Surface.PSN_General2_Surface"))
    (:SurfaceType4
      (LocalVariables|SetSoundVariable "/Game/_Game/Assets/SFX/SFX_GrassFootsteps.SFX_GrassFootsteps")
      (LocalVariables|SetParticleVariable "/Game/A_Surface_Footstep/Niagara_FX/ParticleSystems/PSN_Grass_Surface.PSN_Grass_Surface"))
    (:SurfaceType5
      (LocalVariables|SetSoundVariable "/Game/_Game/Assets/SFX/SFX_WaterFootsteps.SFX_WaterFootsteps")
      (LocalVariables|SetParticleVariable "/Game/A_Surface_Footstep/Niagara_FX/ParticleSystems/PSN_WaterLight_Surface.PSN_WaterLight_Surface")))
  (if (Variables|Default|GetShouldPlaySound)
    (Audio|PlaySoundatLocation (LocalVariables|GetSoundVariable) (LocalVariables|GetSoundSpawnLocation) "0, 0, 0" 1.0 1.0 0.0 0 0 0 0))
  (Niagara|SpawnSystematLocation (LocalVariables|GetParticleVariable) (LocalVariables|GetParticleLocation))
  (return))