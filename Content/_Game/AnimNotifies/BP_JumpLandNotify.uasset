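; Anim notify that plays a surface-specific landing sound when a shooter character lands from a jump.
; On notify, it casts the mesh owner to BP_ShooterCharacter and queries that character's surface type.
; LandSounds maps metal, stone, tile, grass or water to a matching effect, defaulting to tile, and plays it at the owner's location.
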(fn ReceivedNotify
  (params (MeshComp :type Skeletal%20Mesh%20Component%20Object%20Reference) (Animation :type Anim%20Sequence%20Base%20Object%20Reference) (EventReference :type Anim%20Notify%20Event%20Reference%20Structure%20%28by%20ref%29))
  (bind _returnvalue (Components|GetOwner MeshComp))
  (bind _asbp_shooter_character (Utilities|Casting|CastToBP_ShooterCharacter _returnvalue))
  (bind _returnvalue_2 (Class|ShooterCharacter|GetSurfaceType _asbp_shooter_character))
  (CallFunction|LandSounds _returnvalue_2 (Transformation|GetActorLocation _returnvalue))
  (return true))

(fn LandSounds
  (params (Selection :type EPhysicalSurface%20Enum :default "SurfaceType_Default") (Location :type Vector))
  (switch Utilities|FlowControl|Switch|SwitchonEPhysicalSurface Selection
    (:SurfaceType_Default
      (LocalVariables|SetSound "/Game/_Game/Assets/SFX/SFX_LandTile.SFX_LandTile"))
    (:SurfaceType1
      (LocalVariables|SetSound "/Game/_Game/Assets/SFX/SFX_LandMetal.SFX_LandMetal"))
    (:SurfaceType2
      (LocalVariables|SetSound "/Game/_Game/Assets/SFX/SFX_LandConcrete.SFX_LandConcrete"))
    (:SurfaceType3
      (LocalVariables|SetSound "/Game/_Game/Assets/SFX/SFX_LandTile.SFX_LandTile"))
    (:SurfaceType4
      (LocalVariables|SetSound "/Game/_Game/Assets/SFX/SFX_LandGrass.SFX_LandGrass"))
    (:SurfaceType5
      (LocalVariables|SetSound "/Game/_Game/Assets/SFX/SFX_LandWater.SFX_LandWater")))
  (Audio|PlaySoundatLocation (LocalVariables|GetSound) Location "0, 0, 0" 1.0 1.0 0.0 0 0 0 0)
  (return))